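; BP_LapSpliter is a lap-line trigger that counts the player vehicle's laps and detects reverse driving.
; When a component tagged Chassis leaves its box, the dot product of that actor's forward vector and the Arrow's forward vector gives the direction.
; A positive result increments LapCount; otherwise it decrements, with a debug print either way.
; The count always changes on the player 0 BP_SimpleVehicle cached at BeginPlay, whichever actor crossed.
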(event `self.ReceiveBeginPlay`
  (bind _asbp_simple_vehicle (cast `/Game/BluePrints/Vheicle/BP_SimpleVehicle` (`GameplayStatics.GetPlayerPawn` 0))))

(event `self.BoxCollision.OnComponentEndOverlap`
  (params (OverlappedComponent :type "PrimitiveComponent Object Reference") (OtherActor :type "Actor Object Reference") (OtherComp :type "PrimitiveComponent Object Reference") (OtherBodyIndex :type Integer))
  (if (`ActorComponent.ComponentHasTag` OtherComp "Chassis")
    (if (< 0.0 (`KismetMathLibrary.Dot_VectorVector` (`self.GetActorForwardVector` OtherActor) (`SceneComponent.GetForwardVector` (`self.Arrow`))))
      (bind _lapcount (`/Game/BluePrints/Vheicle/BP_SimpleVehicle.LapCount` (stale `self.ReceiveBeginPlay` _asbp_simple_vehicle)))
      (`/Engine/EditorBlueprintResources/StandardMacros.IncrementInt` _lapcount
        (:`  `
          (`KismetSystemLibrary.PrintString` "Lap Added")))
      (else
        (`/Engine/EditorBlueprintResources/StandardMacros.DecrementInt` _lapcount
          (:`  `
            (`KismetSystemLibrary.PrintString` "Reverse Driving!!!")))))))

(fn `UserConstructionScript`)