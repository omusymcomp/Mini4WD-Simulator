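; SplitLaptimer is a collision trigger actor that times laps in a race and prints the results to screen.
; When an actor whose display name ends in "e" leaves its Box, the first pass sets IsRacing, records the game time and prints a start message.
; Each later pass prints the seconds elapsed since the previous one and restarts the timing, reusing Laptime as both timestamp and result.
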(event `self.Box.OnComponentEndOverlap`
  (params (OverlappedComponent :type "PrimitiveComponent Object Reference") (OtherActor :type "Actor Object Reference") (OtherComp :type "PrimitiveComponent Object Reference") (OtherBodyIndex :type Integer))
  (bind _returnvalue (`KismetSystemLibrary.GetGameTimeInSeconds`))
  (if (`KismetStringLibrary.EqualEqual_StrStr` (`KismetStringLibrary.Right` (`KismetSystemLibrary.GetDisplayName` OtherActor) 1) "e")
    (if (`self.isRacing`)
      (bind _output_get (set `self.Laptime` (- _returnvalue (`self.Laptime`))))
      (`KismetSystemLibrary.PrintString` (`KismetStringLibrary.Conv_DoubleToString` _output_get))
      (set `self.Laptime` _returnvalue)
      (else
        (set `self.Laptime` (`KismetSystemLibrary.GetGameTimeInSeconds`))
        (set `self.isRacing` true)
        (`KismetSystemLibrary.PrintString` "start!")))))

(fn `UserConstructionScript`)