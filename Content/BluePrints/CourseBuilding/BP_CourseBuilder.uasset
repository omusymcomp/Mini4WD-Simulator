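; BP_CourseBuilder lets the player build a Mini 4WD course piece by piece, starting with the dummy car's lane.
; Each step spawns every part type at the last transform, showing only the selected one with a blinking material.
; Confirming destroys hidden candidates, restores the kept part's material and records its class and Socket0 transform for chaining.
; CE_GoNext saves transforms, classes and car position to the CurcuitShape slot, then opens CourseRunning.
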(event `self.ReceiveBeginPlay`
  ;[1 1 1] 基準となるスタートストレートとダミーのミニ四駆をスポーン
  (bind _returnvalue (`|SpawnActorFromClass` "/Game/BluePrints/Circuits/PartStraightStart.PartStraightStart_C" (`KismetMathLibrary.MakeTransform` (0.0 0.0 0.0)) "Undefined" "MultiplyWithRoot" null null))
  (set `self.CurcuitBase` _returnvalue)
  (bind _returnvalue_2 (`|SpawnActorFromClass` "/Game/BluePrints/Vheicle/BP_DummyVehicle.BP_DummyVehicle_C" (`SceneComponent.GetRelativeTransform` (`/Game/BluePrints/Circuits/PartStraightStart.SPointM` _returnvalue)) "Undefined" "MultiplyWithRoot" null null))
  (set `self.TargetVehicle` _returnvalue_2)
  ;[1 1 1] 外見を青色にする
  (`PrimitiveComponent.SetMaterial` (`/Game/BluePrints/Vheicle/BP_DummyVehicle.SkeletalMesh` (`self.TargetVehicle`)) 0 "/Game/Models/Circuits/Blinking_DMI.Blinking_DMI"))

(event `EnhancedInput|/Game/BluePrints/Inputs/InputChangeForward`
  (params (ActionValue :type Boolean) (ElapsedSeconds :type "Float (double-precision)") (TriggeredSeconds :type "Float (double-precision)") (InputAction :type "InputAction Object Reference" :default "/Game/BluePrints/Inputs/InputChangeForward.InputChangeForward"))
  (bind _curcuitbase (`self.CurcuitBase`))
  (:`Completed`
    ;[1 1 1] スタート位置を決めるフェーズ？
    (if (== (`self.CircuitNum`) 0)
      ;[1 1 1] 場所決め（範囲内で値変更）
      (if (< (`self.Pos`) 2)
        (`/Engine/EditorBlueprintResources/StandardMacros.IncrementInt` (`self.Pos`)
          (:`  `
            ;[1 1 1] ミニ四駆の位置をPosの値に応じて変更
            (`self.K2_SetActorTransform` (`self.TargetVehicle`) (`|GetArrayItem` (`|MakeArray` (`SceneComponent.GetRelativeTransform` (`/Game/BluePrints/Circuits/PartStraightStart.SPointL` _curcuitbase)) (`SceneComponent.GetRelativeTransform` (`/Game/BluePrints/Circuits/PartStraightStart.SPointM` _curcuitbase)) (`SceneComponent.GetRelativeTransform` (`/Game/BluePrints/Circuits/PartStraightStart.SPointR` _curcuitbase))) (`self.Pos`)) false false :!label _label))))
      (else
        ;[1 1 1] 配列のindexから逸脱しないように値を増やしたり減らしたり
        (`self.SetNextIndex`)
        ;[1 1 1] スポーンしたアクターをActorIndexの値に応じて表示したり消したり
        (for (_array_element _array_index) (`self.SpawnedActors`) :!label _label_2
          (`self.SetActorHiddenInGame` _array_element (!= _array_index (`self.ActorIndex`)))
          (`self.Changed`))))))

(event `CE_spawnMini`
  ;[1 1 1] ミニ四駆の位置をPosの値に応じて変更
  (goto _label))

(event `EnhancedInput|/Game/BluePrints/Inputs/InputChangeBackward`
  (params (ActionValue :type Boolean) (ElapsedSeconds :type "Float (double-precision)") (TriggeredSeconds :type "Float (double-precision)") (InputAction :type "InputAction Object Reference" :default "/Game/BluePrints/Inputs/InputChangeBackward.InputChangeBackward"))
  (:`Completed`
    ;[1 1 1] スタート位置を決めるフェーズ？
    (if (== (`self.CircuitNum`) 0)
      ;[1 1 1] 場所決め（範囲内で値変更）
      (if (< 0 (`self.Pos`))
        (`/Engine/EditorBlueprintResources/StandardMacros.DecrementInt` (`self.Pos`)
          (:`  `
            (goto _label))))
      (else
        ;[1 1 1] 配列のindexから逸脱しないように値を増やしたり減らしたり
        (`self.SetBeforeIndex`)
        (goto _label_2)))))

(event `CE_ActorIndexChanged`
  (goto _label_2))

(event `EnhancedInput|/Game/BluePrints/Inputs/InputDecide`
  (params (ActionValue :type Boolean) (ElapsedSeconds :type "Float (double-precision)") (TriggeredSeconds :type "Float (double-precision)") (InputAction :type "InputAction Object Reference" :default "/Game/BluePrints/Inputs/InputDecide.InputDecide"))
  (:`Completed`
    (`|ExecutionSequence` :!label _label_3
      (:`then_0`
        ;[1 1 1] 表示していないパーツをすべて削除して新しいコースのスポーン位置の基準点を決定
        (`/Engine/EditorBlueprintResources/StandardMacros.IncrementInt` (`self.CircuitNum`)
          (:`  `
            (`self.SetMaterialReset`)
            (for (_array_element _array_index) (`self.SpawnedActors`)
              (if (`Actor.bHidden` _array_element)
                (`self.K2_DestroyActor` _array_element)
                (else
                  (bind _newtransform (`self.GetNextSpawnTransform` _array_index _array_element)) ; 削除せずに残ったパーツのtarget0の場所を読む
                  (`KismetArrayLibrary.Array_Add` (`self.SpawnTransform`) _newtransform)
                  (`KismetArrayLibrary.Array_Add` (`self.SapwnedClass`) (`|GetArrayItem` (`self.ActorsClass`) _array_index)))))
            (`KismetArrayLibrary.Array_Clear` (`self.SpawnedActors`))
            ;[1 1 1] 車の色を戻す
            (`/Engine/EditorBlueprintResources/StandardMacros.DoOnce` false
              (:`Completed`
                (`PrimitiveComponent.SetMaterial` (`/Game/BluePrints/Vheicle/BP_DummyVehicle.SkeletalMesh` (`self.TargetVehicle`)) 0 "/Game/Models/Vheicle/MachineYellow.MachineYellow"))))))
      (:`then_1`
        ;[1 1 1] すべての種類のパーツをスポーンさせてうち一つだけを表示
        (for (_array_element_2 _array_index_2) (`self.ActorsClass`)
          (bind _returnvalue (`|SpawnActorFromClass` _array_element_2 (`|GetArrayItem` (`self.SpawnTransform`) (`KismetArrayLibrary.Array_LastIndex` (`self.SpawnTransform`))) "Undefined" "MultiplyWithRoot" null null))
          (`self.SetActorHiddenInGame` _returnvalue (!= (`self.ActorIndex`) _array_index_2))
          (`KismetArrayLibrary.Array_Add` (`self.SpawnedActors`) _returnvalue)
          (`self.SetMaterialBlue`))))))

(event `CE_DecideFromWidget`
  (goto _label_3))

(event `CE_GoNext`
  (bind _returnvalue (`GameplayStatics.CreateSaveGameObject` "/Game/BluePrints/CourseBuilding/SaveGame_CircuitShape.SaveGame_CircuitShape_C"))
  (bind _output_get (set `self.StoreData` _returnvalue))
  (set `/Game/BluePrints/CourseBuilding/SaveGame_CircuitShape.SpawnPointArray` (`self.SpawnTransform`) _output_get)
  (set `/Game/BluePrints/CourseBuilding/SaveGame_CircuitShape.SpawnedActorClassArray` (`self.SapwnedClass`) _output_get)
  (set `/Game/BluePrints/CourseBuilding/SaveGame_CircuitShape.VehiclePos` (`self.GetTransform` (`self.TargetVehicle`)) _output_get)
  (`GameplayStatics.SaveGameToSlot` (`self.StoreData`) "CurcuitShape")
  (`GameplayStatics.OpenLevelBySoftObjectPtr` "/Game/Levels/CourseRunning.CourseRunning"))

(fn `GetNextSpawnTransform`
  (params (Selection :type Integer) (InputPin :type "Actor Object Reference"))
  (returns (NewTransform :type "Transform Structure"))
  (locals (Return :type "Transform Structure"))
  (switch `int` Selection
    (:`0`
      (bind _aspart_straight (cast `/Game/BluePrints/Circuits/PartStraight` InputPin))
      (set `local.Return` (`SceneComponent.K2_GetComponentToWorld` (`/Game/BluePrints/Circuits/PartStraight.Socket0` _aspart_straight))))
    (:`1`
      (bind _aspart_45r (cast `/Game/BluePrints/Circuits/Part45R` InputPin))
      (set `local.Return` (`SceneComponent.K2_GetComponentToWorld` (`/Game/BluePrints/Circuits/Part45R.Socket0` _aspart_45r))))
    (:`2`
      (bind _aspart_45l (cast `/Game/BluePrints/Circuits/Part45L` InputPin))
      (set `local.Return` (`SceneComponent.K2_GetComponentToWorld` (`/Game/BluePrints/Circuits/Part45L.Socket0` _aspart_45l))))
    (:`3`
      (bind _aspart_wave_r (cast `/Game/BluePrints/Circuits/PartWaveR` InputPin))
      (set `local.Return` (`SceneComponent.K2_GetComponentToWorld` (`/Game/BluePrints/Circuits/PartWaveR.Socket0` _aspart_wave_r))))
    (:`4`
      (bind _aspart_wave_l (cast `/Game/BluePrints/Circuits/PartWaveL` InputPin))
      (set `local.Return` (`SceneComponent.K2_GetComponentToWorld` (`/Game/BluePrints/Circuits/PartWaveL.Socket0` _aspart_wave_l))))
    (:`5`
      (bind _aspart_slope_up (cast `/Game/BluePrints/Circuits/PartSlopeUp` InputPin))
      (set `local.Return` (`SceneComponent.K2_GetComponentToWorld` (`/Game/BluePrints/Circuits/PartSlopeUp.Socket0` _aspart_slope_up))))
    (:`6`
      (bind _aspart_slope_down (cast `/Game/BluePrints/Circuits/PartSlopeDown` InputPin))
      (set `local.Return` (`SceneComponent.K2_GetComponentToWorld` (`/Game/BluePrints/Circuits/PartSlopeDown.Socket0` _aspart_slope_down))))
    (:`7`
      (bind _aspart_lc (cast `/Game/BluePrints/Circuits/PartLC` InputPin))
      (set `local.Return` (`SceneComponent.K2_GetComponentToWorld` (`/Game/BluePrints/Circuits/PartLC.Socket0` _aspart_lc))))
    (:`8`
      (bind _aspart_bank (cast `/Game/BluePrints/Circuits/PartBank` InputPin))
      (set `local.Return` (`SceneComponent.K2_GetComponentToWorld` (`/Game/BluePrints/Circuits/PartBank.Socket0` _aspart_bank))))
    (:`9`
      (bind _aspart_jump (cast `/Game/BluePrints/Circuits/PartJump` InputPin))
      (set `local.Return` (`SceneComponent.K2_GetComponentToWorld` (`/Game/BluePrints/Circuits/PartJump.Socket0` _aspart_jump)))))
  (return (`local.Return`)))

(fn `SetBeforeIndex`
  (returns (NewActorIndex :type Integer))
  (if (< 0 (`self.ActorIndex`))
    (`/Engine/EditorBlueprintResources/StandardMacros.DecrementInt` (`self.ActorIndex`)
      (:`  `
        _))
    (else
      (set `self.ActorIndex` (`KismetArrayLibrary.Array_LastIndex` (`self.ActorsClass`)))))
  (return (`self.ActorIndex`)))

(fn `SetMaterialBlue`
  (for _array_element (`self.SpawnedActors`)
    (bind _aspart_straight (cast `/Game/BluePrints/Circuits/PartStraight` _array_element)
      (:`then`
        (`PrimitiveComponent.SetMaterial` (`/Game/BluePrints/Circuits/PartStraight.StaticMesh` _aspart_straight) 0 "/Game/Models/Circuits/Blinking_DMI.Blinking_DMI"))
      (:`CastFailed`
        (bind _aspart_45r (cast `/Game/BluePrints/Circuits/Part45R` _array_element)
          (:`then`
            (`PrimitiveComponent.SetMaterial` (`/Game/BluePrints/Circuits/Part45R.StaticMesh` _aspart_45r) 0 "/Game/Models/Circuits/Blinking_DMI.Blinking_DMI"))
          (:`CastFailed`
            (bind _aspart_45l (cast `/Game/BluePrints/Circuits/Part45L` _array_element)
              (:`then`
                (`PrimitiveComponent.SetMaterial` (`/Game/BluePrints/Circuits/Part45L.StaticMesh` _aspart_45l) 0 "/Game/Models/Circuits/Blinking_DMI.Blinking_DMI"))
              (:`CastFailed`
                (bind _aspart_wave_r (cast `/Game/BluePrints/Circuits/PartWaveR` _array_element)
                  (:`then`
                    (`PrimitiveComponent.SetMaterial` (`/Game/BluePrints/Circuits/PartWaveR.StaticMesh` _aspart_wave_r) 0 "/Game/Models/Circuits/Blinking_DMI.Blinking_DMI"))
                  (:`CastFailed`
                    (bind _aspart_wave_l (cast `/Game/BluePrints/Circuits/PartWaveL` _array_element)
                      (:`then`
                        (`PrimitiveComponent.SetMaterial` (`/Game/BluePrints/Circuits/PartWaveL.StaticMesh` _aspart_wave_l) 0 "/Game/Models/Circuits/Blinking_DMI.Blinking_DMI"))
                      (:`CastFailed`
                        (bind _aspart_slope_up (cast `/Game/BluePrints/Circuits/PartSlopeUp` _array_element)
                          (:`then`
                            (`PrimitiveComponent.SetMaterial` (`/Game/BluePrints/Circuits/PartSlopeUp.StaticMesh` _aspart_slope_up) 0 "/Game/Models/Circuits/Blinking_DMI.Blinking_DMI"))
                          (:`CastFailed`
                            (bind _aspart_slope_down (cast `/Game/BluePrints/Circuits/PartSlopeDown` _array_element)
                              (:`then`
                                (`PrimitiveComponent.SetMaterial` (`/Game/BluePrints/Circuits/PartSlopeDown.StaticMesh` _aspart_slope_down) 0 "/Game/Models/Circuits/Blinking_DMI.Blinking_DMI"))
                              (:`CastFailed`
                                (bind _aspart_lc (cast `/Game/BluePrints/Circuits/PartLC` _array_element)
                                  (:`then`
                                    (`PrimitiveComponent.SetMaterial` (`/Game/BluePrints/Circuits/PartLC.StaticMesh` _aspart_lc) 0 "/Game/Models/Circuits/Blinking_DMI.Blinking_DMI"))
                                  (:`CastFailed`
                                    (bind _aspart_bank (cast `/Game/BluePrints/Circuits/PartBank` _array_element)
                                      (:`then`
                                        (`PrimitiveComponent.SetMaterial` (`/Game/BluePrints/Circuits/PartBank.StaticMesh` _aspart_bank) 0 "/Game/Models/Circuits/Blinking_DMI.Blinking_DMI"))
                                      (:`CastFailed`
                                        (bind _aspart_jump (cast `/Game/BluePrints/Circuits/PartJump` _array_element))
                                        (`PrimitiveComponent.SetMaterial` (`/Game/BluePrints/Circuits/PartJump.StaticMesh` _aspart_jump) 0 "/Game/Models/Circuits/Blinking_DMI.Blinking_DMI")))))))))))))))))))))

(fn `SetMaterialReset`
  (for _array_element (`self.SpawnedActors`)
    (bind _aspart_straight (cast `/Game/BluePrints/Circuits/PartStraight` _array_element)
      (:`then`
        (`PrimitiveComponent.SetMaterial` (`/Game/BluePrints/Circuits/PartStraight.StaticMesh` _aspart_straight) 0 "/Game/Models/Circuits/Course_white.Course_white"))
      (:`CastFailed`
        (bind _aspart_45r (cast `/Game/BluePrints/Circuits/Part45R` _array_element)
          (:`then`
            (`PrimitiveComponent.SetMaterial` (`/Game/BluePrints/Circuits/Part45R.StaticMesh` _aspart_45r) 0 "/Game/Models/Circuits/Course_red.Course_red"))
          (:`CastFailed`
            (bind _aspart_45l (cast `/Game/BluePrints/Circuits/Part45L` _array_element)
              (:`then`
                (`PrimitiveComponent.SetMaterial` (`/Game/BluePrints/Circuits/Part45L.StaticMesh` _aspart_45l) 0 "/Game/Models/Circuits/Course_red.Course_red"))
              (:`CastFailed`
                (bind _aspart_wave_r (cast `/Game/BluePrints/Circuits/PartWaveR` _array_element)
                  (:`then`
                    (`PrimitiveComponent.SetMaterial` (`/Game/BluePrints/Circuits/PartWaveR.StaticMesh` _aspart_wave_r) 0 "/Game/Models/Circuits/Course_white.Course_white"))
                  (:`CastFailed`
                    (bind _aspart_wave_l (cast `/Game/BluePrints/Circuits/PartWaveL` _array_element)
                      (:`then`
                        (`PrimitiveComponent.SetMaterial` (`/Game/BluePrints/Circuits/PartWaveL.StaticMesh` _aspart_wave_l) 0 "/Game/Models/Circuits/Course_white.Course_white"))
                      (:`CastFailed`
                        (bind _aspart_slope_up (cast `/Game/BluePrints/Circuits/PartSlopeUp` _array_element)
                          (:`then`
                            (`PrimitiveComponent.SetMaterial` (`/Game/BluePrints/Circuits/PartSlopeUp.StaticMesh` _aspart_slope_up) 0 "/Game/Models/Circuits/Course_red.Course_red"))
                          (:`CastFailed`
                            (bind _aspart_slope_down (cast `/Game/BluePrints/Circuits/PartSlopeDown` _array_element)
                              (:`then`
                                (`PrimitiveComponent.SetMaterial` (`/Game/BluePrints/Circuits/PartSlopeDown.StaticMesh` _aspart_slope_down) 0 "/Game/Models/Circuits/Course_red.Course_red"))
                              (:`CastFailed`
                                (bind _aspart_lc (cast `/Game/BluePrints/Circuits/PartLC` _array_element)
                                  (:`then`
                                    (`PrimitiveComponent.SetMaterial` (`/Game/BluePrints/Circuits/PartLC.StaticMesh` _aspart_lc) 0 "/Game/Models/Circuits/Course_white.Course_white"))
                                  (:`CastFailed`
                                    (bind _aspart_bank (cast `/Game/BluePrints/Circuits/PartBank` _array_element)
                                      (:`then`
                                        (`PrimitiveComponent.SetMaterial` (`/Game/BluePrints/Circuits/PartBank.StaticMesh` _aspart_bank) 0 "/Game/Models/Circuits/Course_red.Course_red"))
                                      (:`CastFailed`
                                        (bind _aspart_jump (cast `/Game/BluePrints/Circuits/PartJump` _array_element))
                                        (`PrimitiveComponent.SetMaterial` (`/Game/BluePrints/Circuits/PartJump.StaticMesh` _aspart_jump) 0 "/Game/Models/Circuits/Course_white.Course_white")))))))))))))))))))))

(fn `SetNextIndex`
  (returns (NewActorIndex :type Integer))
  (if (< (`self.ActorIndex`) (`KismetArrayLibrary.Array_LastIndex` (`self.ActorsClass`)))
    (`/Engine/EditorBlueprintResources/StandardMacros.IncrementInt` (`self.ActorIndex`)
      (:`  `
        _))
    (else
      (set `self.ActorIndex` 0)))
  (return (`self.ActorIndex`)))

(fn `UserConstructionScript`)